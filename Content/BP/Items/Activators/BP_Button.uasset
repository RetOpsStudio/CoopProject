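; BP_Button is an activator item whose Button mesh changes material to show whether it is activated.
; On the server, begin-activate calls a multicast that applies M_Bush, while cancel and end both call a multicast that restores M_AssetPlatform.
; Authority checks limit the calls to the server so the multicasts carry the visual change to clients.
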(event `MulticastActivate`
  (`PrimitiveComponent.SetMaterial` (`self.Button`) 0 "/Game/StarterContent/Props/Materials/M_Bush.M_Bush"))

(event `self.OnItemBeginActivateBP`
  (`/Engine/EditorBlueprintResources/ActorMacros.Switch Has Authority`
    (:`Authority`
      (`self.MulticastActivate`))))

(event `MulticastDeactivate`
  (`PrimitiveComponent.SetMaterial` (`self.Button`) 0 "/Game/StarterContent/Materials/M_AssetPlatform.M_AssetPlatform"))

(event `self.OnItemCancelActivateBP`
  (`/Engine/EditorBlueprintResources/ActorMacros.Switch Has Authority` :!label _label
    (:`Authority`
      (`self.MulticastDeactivate`))))

(event `self.OnItemEndActivateBP`
  (goto _label))

(fn `UserConstructionScript`)